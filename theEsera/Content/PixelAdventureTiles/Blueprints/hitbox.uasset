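; Hitbox hazard actor that damages the 2D side-scroller player character on contact.
; Overlapping its Rrr component subtracts a fixed amount from the character's current health and prints the new value.
; Exact-equality health checks, rather than a threshold, decide when to print "dead" and add the Gameover widget to the viewport, which happens only when remaining health equals one.
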(event OnComponentBeginOverlap(rrr)
  (params (OverlappedComponent :type Primitive%20Component%20Object%20Reference) (OtherActor :type Actor%20Object%20Reference) (OtherComp :type Primitive%20Component%20Object%20Reference) (OtherBodyIndex :type Integer) (bFromSweep :type Boolean) (SweepResult :type Hit%20Result%20Structure%20%28by%20ref%29))
  (bind _asbp_2dside_scroller_character (Utilities|Casting|CastToBP_2DSideScrollerCharacter OtherActor))
  (Variables|/Game/PixelAdventureTiles/Blueprints/BP_2DSideScrollerCharacter.BP_2DSideScrollerCharacter_C|Sethealth%20current _asbp_2dside_scroller_character (- (Variables|/Game/PixelAdventureTiles/Blueprints/BP_2DSideScrollerCharacter.BP_2DSideScrollerCharacter_C|Gethealth%20current _asbp_2dside_scroller_character) 4.0))
  (Development|PrintString (Utilities|String|ToString(Float) (Variables|/Game/PixelAdventureTiles/Blueprints/BP_2DSideScrollerCharacter.BP_2DSideScrollerCharacter_C|Gethealth%20current _asbp_2dside_scroller_character)))
  (if (not (== 3.0 (Variables|/Game/PixelAdventureTiles/Blueprints/BP_2DSideScrollerCharacter.BP_2DSideScrollerCharacter_C|Gethealth%20current _asbp_2dside_scroller_character)))
    (if (== 0.0 (- (Variables|/Game/PixelAdventureTiles/Blueprints/BP_2DSideScrollerCharacter.BP_2DSideScrollerCharacter_C|Gethealth%20current _asbp_2dside_scroller_character) 1.0))
      (Development|PrintString "dead")
      (bind _returnvalue (UserInterface|CreateWidget "/Game/PixelAdventureTiles/widgets/gameover.gameover_C"))
      (UserInterface|Viewport|AddtoViewport _returnvalue 0))))

(event EventBeginPlay)

(event Collision|EventActorBeginOverlap
  (params (OtherActor :type Actor%20Object%20Reference)))

(event EventTick
  (params (DeltaSeconds :type Float%20%28single-precision%29)))

(fn ConstructionScript)