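; Lift actor in PixelAdventureTiles that moves continuously up and down along the Z axis.
; Each Tick offsets the render component's world location by the normalized direction vector, scaled by Speed and delta time, without sweeping.
; A Delay on the same Tick chain feeds a FlipFlop that reverses the direction every four seconds, so travel is timed rather than bound to endpoints.
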(event EventBeginPlay)

(event Collision|EventActorBeginOverlap
  (params (OtherActor :type Actor%20Object%20Reference)))

(event EventTick
  (params (DeltaSeconds :type Float%20%28single-precision%29))
  (bind _rendercomponent (Variables|Default|GetRenderComponent))
  (bind _returnvalue (Transformation|GetWorldTransform _rendercomponent))
  (bind (_location _rotation _scale) (Math|Transform|BreakTransform _returnvalue))
  (Transformation|SetActorTransform (Math|Transform|MakeTransform (+ (* (Math|Vector|Normalize (Variables|Default|Gettglocation)) (* (Utilities|Time|GetWorldDeltaSeconds) (Variables|Default|Getspeed))) _location) _rotation _scale))
  (Utilities|FlowControl|Delay 4.0)
  (Utilities|FlowControl|FlipFlop
    (:A
      (Variables|Default|Settglocation "0.000000,0.000000,80.000000"))
    (:B
      (Variables|Default|Settglocation "0.000000,0.000000,-80.000000"))))

(fn ConstructionScript)