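; Side-scroller chest pickup that can drop loot and destroys itself when the player character class overlaps its R component.
; The overlap runs a DropLoot loop with a randomized bound that always resolves to a single pass.
; DropLoot traces down to place the spawn at the hit location, picking randomly from class slots where only the red potion is filled, so some rolls have no item.
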(event OnComponentBeginOverlap(r)
  (params (OverlappedComponent :type Primitive%20Component%20Object%20Reference) (OtherActor :type Actor%20Object%20Reference) (OtherComp :type Primitive%20Component%20Object%20Reference) (OtherBodyIndex :type Integer) (bFromSweep :type Boolean) (SweepResult :type Hit%20Result%20Structure%20%28by%20ref%29))
  (Utilities|Casting|CastToBP_2DSideScrollerCharacter OtherActor)
  (for _index (range 0 (Math|Random|RandomInteger 1))
    (CallFunction|DropLoot))
  (Actor|DestroyActor))

(event Custom|DropLoot
  (bind _returnvalue (Transformation|GetActorLocation))
  (bind _outhit (Collision|LineTraceByChannel _returnvalue (- _returnvalue "0,0.000000,300.000000") "TraceTypeQuery1" false (Utilities|Array|MakeArray (Game|GetPlayerCharacter 0)) "None"))
  (Game|SpawnActorfromClass (Utilities|Select :Index (Math|Random|RandomInteger 3) :Option%200 "/Game/PixelAdventureTiles/Blueprints/SP_PotionRed_Blueprint.SP_PotionRed_Blueprint_C" :Option%201 0 :Option%202 0 :Option%203 0) (Math|Transform|MakeTransform (.Location (Collision|BreakHitResult _outhit))) "Undefined" 0 0))

(event EventBeginPlay)

(event Collision|EventActorBeginOverlap
  (params (OtherActor :type Actor%20Object%20Reference)))

(event EventTick
  (params (DeltaSeconds :type Float%20%28single-precision%29)))

(fn ConstructionScript)