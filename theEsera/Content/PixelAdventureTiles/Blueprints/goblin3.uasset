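; Goblin enemy for a 2D side-scroller that takes arrow hits and adds to the player's kill count.
; It patrols via InterpToMovement between relative PointA and PointB, and Tick also shifts it along local negative X while CanMove, set through OverlappedPlayer, is true.
; BP_Arrow overlaps decrement health; at zero it shows an explosion flipbook, plays a sound, then after a delay destroys itself and increments the character's Kill.
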(event Collision|EventActorBeginOverlap
  (params (OtherActor :type Actor%20Object%20Reference))
  (Utilities|Casting|CastToBP_Arrow OtherActor)
  (bind _output_get (Variables|Default|Sethealth-mons3 (- (Variables|Default|Gethealth-mons3) 1.0)))
  (Development|PrintString (Utilities|String|ToString(Float) (Variables|Default|Gethealth-mons3)))
  (if (== 0.0 _output_get)
    (Sprite|SetFlipbook (Variables|Default|GetPaperFlipbook) "/Game/PixelAdventureTiles/Flipbooks/FB_Explosion.FB_Explosion")
    (Audio|PlaySoundatLocation "/Engine/VREditor/Sounds/UI/Teleport_Committed.Teleport_Committed" "0, 0, 0" "0, 0, 0" 1.0 1.0 0.0 0 0 0)
    (Utilities|FlowControl|Delay 0.3)
    (Actor|DestroyActor)
    (bind _returnvalue (Actor|GetActorOfClass "/Game/PixelAdventureTiles/Blueprints/BP_2DSideScrollerCharacter.BP_2DSideScrollerCharacter_C"))
    (Variables|/Game/PixelAdventureTiles/Blueprints/BP_2DSideScrollerCharacter.BP_2DSideScrollerCharacter_C|Setkill _returnvalue (+ (Variables|/Game/PixelAdventureTiles/Blueprints/BP_2DSideScrollerCharacter.BP_2DSideScrollerCharacter_C|Getkill _returnvalue) 1.0))))

(event EventTick
  (params (DeltaSeconds :type Float%20%28single-precision%29))
  (if (Variables|Default|GetcanMove)
    (Transformation|AddActorLocalOffset "-3.000000, 0,0.000000" false false)))

(event EventBeginPlay)

(fn ConstructionScript
  (Variables|/Script/Engine.InterpToMovementComponent|SetControlPoints (Variables|Default|GetInterpToMovement) (Utilities|Array|MakeArray (Utilities|Struct|MakeInterpControlPoint (Variables|Default|GetPointA) true) (Utilities|Struct|MakeInterpControlPoint (Variables|Default|GetPointB) true))))

(fn OverlappedPlayer
  (params (BeginOverlap :type Boolean))
  (Variables|Default|SetcanMove BeginOverlap))