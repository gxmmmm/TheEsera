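; Treasure chest for the 2D side-scroller that serves as the win condition once the player has enough kills.
; On actor overlap, it casts to the side-scroller character and checks its Kill count against a fixed threshold.
; Success plays a sound, swaps the flipbook to the chest animation, then shows the Win widget after delays.
; Failure plays an invalid-action sound and briefly reveals the character's KillMore prompt.
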(event OnComponentHit(Box)
  (params (HitComponent :type Primitive%20Component%20Object%20Reference) (OtherActor :type Actor%20Object%20Reference) (OtherComp :type Primitive%20Component%20Object%20Reference) (NormalImpulse :type Vector :default "0, 0, 0") (Hit :type Hit%20Result%20Structure%20%28by%20ref%29)))

(event OnComponentBeginOverlap(Box)
  (params (OverlappedComponent :type Primitive%20Component%20Object%20Reference) (OtherActor :type Actor%20Object%20Reference) (OtherComp :type Primitive%20Component%20Object%20Reference) (OtherBodyIndex :type Integer) (bFromSweep :type Boolean) (SweepResult :type Hit%20Result%20Structure%20%28by%20ref%29)))

(event EventBeginPlay)

(event Collision|EventActorBeginOverlap
  (params (OtherActor :type Actor%20Object%20Reference))
  (bind _asbp_2dside_scroller_character (Utilities|Casting|CastToBP_2DSideScrollerCharacter OtherActor))
  (Development|PrintString "Hello")
  (if (>= (Variables|/Game/PixelAdventureTiles/Blueprints/BP_2DSideScrollerCharacter.BP_2DSideScrollerCharacter_C|Getkill _asbp_2dside_scroller_character) 8.0)
    (Audio|PlaySoundatLocation "/Engine/VREditor/Sounds/UI/Dockable_Window_Open.Dockable_Window_Open" "0, 0, 0" "0, 0, 0" 1.0 1.0 0.0 0 0 0)
    (Utilities|FlowControl|Delay 0.3)
    (Sprite|SetFlipbook (Variables|Default|GetPaperFlipbook) "/Game/PixelAdventureTiles/Flipbooks/FB_Chest.FB_Chest")
    (Utilities|FlowControl|Delay 3.0)
    (bind _returnvalue (UserInterface|CreateWidget "/Game/PixelAdventureTiles/widgets/win.win_C"))
    (UserInterface|Viewport|AddtoViewport _returnvalue 0)
    (else
      (Audio|PlaySoundatLocation "/Engine/VREditor/Sounds/UI/Invalid_Action.Invalid_Action" "0, 0, 0" "0, 0, 0" 1.0 1.0 0.0 0 0 0)
      (Variables|/Game/PixelAdventureTiles/Blueprints/BP_2DSideScrollerCharacter.BP_2DSideScrollerCharacter_C|Setkill%20more _asbp_2dside_scroller_character "Visible")
      (Utilities|FlowControl|Delay 3.0)
      (Variables|/Game/PixelAdventureTiles/Blueprints/BP_2DSideScrollerCharacter.BP_2DSideScrollerCharacter_C|Setkill%20more _asbp_2dside_scroller_character "Hidden"))))

(event EventTick
  (params (DeltaSeconds :type Float%20%28single-precision%29)))

(fn ConstructionScript)