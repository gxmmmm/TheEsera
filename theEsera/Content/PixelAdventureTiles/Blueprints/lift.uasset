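; A lift actor that travels back and forth along the vertical axis.
; Each Tick moves it along the normalized Direction by Speed times delta time, offsetting from the RenderComponent's transform without sweep.
; A Delay in the same Tick chain acts as a repeating three-second timer, driving a FlipFlop that alternates Direction between up and down.
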(event EventTick
  (params (DeltaSeconds :type Float%20%28single-precision%29))
  (bind _rendercomponent (Variables|Default|GetRenderComponent))
  (bind _returnvalue (Transformation|GetWorldTransform _rendercomponent))
  (bind (_location _rotation _scale) (Math|Transform|BreakTransform _returnvalue))
  (Transformation|SetActorTransform (Math|Transform|MakeTransform (+ (* (Math|Vector|Normalize (Variables|Default|GetDirection)) (* (Utilities|Time|GetWorldDeltaSeconds) (Variables|Default|GetSpeed))) _location) _rotation _scale))
  (Utilities|FlowControl|Delay 3.0)
  (Utilities|FlowControl|FlipFlop
    (:A
      (Variables|Default|SetDirection "0,0.000000,80.000000"))
    (:B
      (Variables|Default|SetDirection "0,0.000000,-80.000000"))))

(fn ConstructionScript)