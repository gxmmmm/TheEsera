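; Goblin enemy actor that moves between two editable points and dies when hit by a BP_Arrow.
; The construction script turns PointA and PointB into relative InterpToMovement control points.
; An arrow overlap decrements and prints health, shows an explosion flipbook, then destroys the goblin after a delay regardless of health and increments the arrow's Kill count.
; OverlappedPlayer sets CanMove from its overlap flag.
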(event Collision|EventActorBeginOverlap
  (params (OtherActor :type Actor%20Object%20Reference))
  (bind _asbp_arrow (Utilities|Casting|CastToBP_Arrow OtherActor))
  (Variables|Default|Sethealth-mons1 (- (Variables|Default|Gethealth-mons1) 1.0))
  (Development|PrintString (Utilities|String|ToString(Float) (Variables|Default|Gethealth-mons1)))
  (Sprite|SetFlipbook (Variables|Default|GetPaperFlipbook) "/Game/PixelAdventureTiles/Flipbooks/FB_Explosion.FB_Explosion")
  (Utilities|FlowControl|Delay 0.5)
  (Actor|DestroyActor)
  (Variables|/Game/PixelAdventureTiles/Blueprints/BP_Arrow.BP_Arrow_C|Setkill _asbp_arrow (+ (Variables|/Game/PixelAdventureTiles/Blueprints/BP_Arrow.BP_Arrow_C|Getkill _asbp_arrow) 1.0)))

(fn ConstructionScript
  (Variables|/Script/Engine.InterpToMovementComponent|SetControlPoints (Variables|Default|GetInterpToMovement) (Utilities|Array|MakeArray (Utilities|Struct|MakeInterpControlPoint (Variables|Default|GetPointA) true) (Utilities|Struct|MakeInterpControlPoint (Variables|Default|GetPointB) true))))

(fn OverlappedPlayer
  (params (BeginOverlap :type Boolean))
  (Variables|Default|SetcanMove BeginOverlap))