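; BP_Bat_Blueprint is a flying bat enemy for a 2D side-scroller, animated with flipbooks.
; Each Tick moves it along X by SpeedX while a sine of an incrementing counter bobs it on Z, using a swept teleport move.
; An overlapping BP_Arrow decrements and prints Healthmons1, then swaps in the explosion flipbook and destroys the bat after a short delay, regardless of remaining health.
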(event Collision|EventActorBeginOverlap
  (params (OtherActor :type Actor%20Object%20Reference))
  (Utilities|Casting|CastToBP_Arrow OtherActor)
  (Variables|Default|Sethealth-mons1 (- (Variables|Default|Gethealth-mons1) 1.0))
  (Development|PrintString (Utilities|String|ToString(Float) (Variables|Default|Gethealth-mons1)))
  (Sprite|SetFlipbook (Variables|Default|GetRenderComponent) "/Game/PixelAdventureTiles/Flipbooks/FB_Explosion.FB_Explosion")
  (Utilities|FlowControl|Delay 0.5)
  (Actor|DestroyActor))

(event EventTick
  (params (DeltaSeconds :type Float%20%28single-precision%29))
  (bind _returnvalue (Transformation|GetActorLocation))
  ;[1 1 1] Sinusoidal movement
  (Math|Integer|IncrementInt (Variables|Default|GetsinIncrement)
    (:%20%20
      (Transformation|SetActorLocation (Math|Vector|MakeVector (+ (.x _returnvalue) (Variables|Default|GetspeedX)) 0.0 (+ (.z _returnvalue) (* (Math|Trig|Sin(Degrees) (Math|Float|MultiplybyPi (Math|Conversions|ToFloat(Integer) (Variables|Default|GetsinIncrement)))) 3.0))) true true))))

(event EventBeginPlay)

(fn ConstructionScript)