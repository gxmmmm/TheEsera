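; Goblin enemy Blueprint that moves along an InterpToMovement path between two relative points, PointA and PointB, set in the construction script.
; An overlap with BP_Arrow decrements and prints its health, then plays an explosion flipbook and sound regardless of remaining health.
; After a short delay it destroys itself and increments the Kill count on BP_2DSideScrollerCharacter.
; A separate OverlappedPlayer function sets CanMove from its overlap flag.
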(event Collision|EventActorBeginOverlap
  (params (OtherActor :type Actor%20Object%20Reference))
  (Utilities|Casting|CastToBP_Arrow OtherActor)
  (Variables|Default|Sethealth-mons1 (- (Variables|Default|Gethealth-mons1) 1.0))
  (Development|PrintString (Utilities|String|ToString(Float) (Variables|Default|Gethealth-mons1)))
  (Sprite|SetFlipbook (Variables|Default|GetPaperFlipbook) "/Game/PixelAdventureTiles/Flipbooks/FB_Explosion.FB_Explosion")
  (Audio|PlaySoundatLocation "/Engine/VREditor/Sounds/UI/Teleport_Committed.Teleport_Committed" "0, 0, 0" "0, 0, 0" 1.0 1.0 0.0 0 0 0)
  (Utilities|FlowControl|Delay 0.3)
  (Actor|DestroyActor)
  (bind _returnvalue (Actor|GetActorOfClass "/Game/PixelAdventureTiles/Blueprints/BP_2DSideScrollerCharacter.BP_2DSideScrollerCharacter_C"))
  (Variables|/Game/PixelAdventureTiles/Blueprints/BP_2DSideScrollerCharacter.BP_2DSideScrollerCharacter_C|Setkill _returnvalue (+ (Variables|/Game/PixelAdventureTiles/Blueprints/BP_2DSideScrollerCharacter.BP_2DSideScrollerCharacter_C|Getkill _returnvalue) 1.0)))

(fn ConstructionScript
  (Variables|/Script/Engine.InterpToMovementComponent|SetControlPoints (Variables|Default|GetInterpToMovement) (Utilities|Array|MakeArray (Utilities|Struct|MakeInterpControlPoint (Variables|Default|GetPointA) true) (Utilities|Struct|MakeInterpControlPoint (Variables|Default|GetPointB) true))))

(fn OverlappedPlayer
  (params (BeginOverlap :type Boolean))
  (Variables|Default|SetcanMove BeginOverlap))